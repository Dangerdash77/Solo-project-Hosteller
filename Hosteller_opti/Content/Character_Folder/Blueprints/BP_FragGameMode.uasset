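; Game mode that drives the layered, progression-based soundtrack through a single master audio component, created and cached on BeginPlay.
; Pathway, four altar and boss sequence events fire Set and Reset trigger parameters on it, building up stems, swapping to piano sections, then switching to boss music.
; Two volume events pass sound and SFX gain to the same component as float parameters, printing each value.
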(event `self.ReceiveBeginPlay`
  (bind _returnvalue (`AddComponent|NODE_AddAudioComponent-0`))
  (set `self.MS_MasterReference` _returnvalue))

(event `Trigger_Altar_1`
  (bind _ms_masterreference (`self.MS_MasterReference`))
  (`AudioParameterControllerInterface.SetTriggerParameter` _ms_masterreference "G_SetBass")
  (`AudioParameterControllerInterface.SetTriggerParameter` _ms_masterreference "G_SetDistortedFoley"))

(event `Trigger_Altar_2`
  (bind _ms_masterreference (`self.MS_MasterReference`))
  (`AudioParameterControllerInterface.SetTriggerParameter` _ms_masterreference "G_SetPads")
  (`AudioParameterControllerInterface.SetTriggerParameter` _ms_masterreference "G_SetPadsV2")
  (`AudioParameterControllerInterface.SetTriggerParameter` _ms_masterreference "G_SetWhimper")
  (`AudioParameterControllerInterface.SetTriggerParameter` _ms_masterreference "G_SetKanglings"))

(event `Trigger_Altar_3`
  (bind _ms_masterreference (`self.MS_MasterReference`))
  (`|ExecutionSequence`
    (:`then_0`
      (`AudioParameterControllerInterface.SetTriggerParameter` _ms_masterreference "G_ResetPadsV2")
      (`AudioParameterControllerInterface.SetTriggerParameter` _ms_masterreference "G_ResetBass")
      (`AudioParameterControllerInterface.SetTriggerParameter` _ms_masterreference "G_ResetDistortedFoley")
      (`AudioParameterControllerInterface.SetTriggerParameter` _ms_masterreference "G_ResetKanglings"))
    (:`then_1`
      (`AudioParameterControllerInterface.SetTriggerParameter` _ms_masterreference "G_SetPianoA"))))

(event `Trigger_Altar_4`
  (bind _ms_masterreference (`self.MS_MasterReference`))
  (`|ExecutionSequence`
    (:`then_0`
      (`AudioParameterControllerInterface.SetTriggerParameter` _ms_masterreference "G_ResetPianoA")
      (`AudioParameterControllerInterface.SetTriggerParameter` _ms_masterreference "G_ResetWhimper")
      (`AudioParameterControllerInterface.SetTriggerParameter` _ms_masterreference "G_ResetPads"))
    (:`then_1`
      (`AudioParameterControllerInterface.SetTriggerParameter` _ms_masterreference "G_SetPianoB"))))

(event `VolumeControl`
  (params (Volume :type "Float (double-precision)"))
  (`KismetSystemLibrary.PrintString` (`KismetStringLibrary.Conv_DoubleToString` Volume))
  (`AudioComponent.SetFloatParameter` (`self.MS_MasterReference`) "G_SoundGain" Volume))

(event `SFXControl`
  (params (Volume :type "Float (double-precision)"))
  (`KismetSystemLibrary.PrintString` (`KismetStringLibrary.Conv_DoubleToString` Volume))
  (`AudioParameterControllerInterface.SetFloatParameter` (`self.MS_MasterReference`) "G_SFXGain" Volume))

(event `Trigger_Boss_Sequence`
  (bind _ms_masterreference (`self.MS_MasterReference`))
  (`|ExecutionSequence`
    (:`then_0`
      (`AudioParameterControllerInterface.SetTriggerParameter` _ms_masterreference "G_ResetPianoB")
      (`AudioParameterControllerInterface.SetTriggerParameter` _ms_masterreference "G_ResetCore"))
    (:`then_1`
      (`AudioParameterControllerInterface.SetTriggerParameter` _ms_masterreference "G_SetStartBoss"))))

(event `TriggerPathway`
  (`AudioParameterControllerInterface.SetTriggerParameter` (`self.MS_MasterReference`) "G_SetCore"))

(fn `UserConstructionScript`)