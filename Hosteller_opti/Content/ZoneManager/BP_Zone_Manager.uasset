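; Zone manager that turns player zone events into game mode triggers for the pathway, altar and church boss sequences.
; Binds to enter, leave, finish and unlatch events, logging entries and exits and destroying a finished zone's mapped volume.
; All altar zones share one branch that advances the altar stages in order, regardless of which altar is entered.
; A latch blocks further altar advances until the unlatched event clears it.
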(event `self.ReceiveBeginPlay`
  (`|ExecutionSequence`
    (:`then_0`
      (bind _asbp_frag_game_mode (cast `/Game/Character_Folder/Blueprints/BP_FragGameMode` (`GameplayStatics.GetGameMode`)))
      (set `self.GameMode Reference` _asbp_frag_game_mode))
    (:`then_1`
      (add `self.UnlatchedDispatcher` (delegate `Unlatched`))
      (add `self.PlayerEntered` (`|CreateDelegate` :!event `PlayerEnteredResponse`))
      (add `self.PlayerLeave` (`|CreateDelegate` :!event `PlayerLeaveResponse`))
      (add `self.FinishZone` (`|CreateDelegate` :!event `FinishZoneResponse`)))))

(event `Unlatched`
  (set `self.Latched` false))

(event `PlayerLeaveResponse`
  (`KismetSystemLibrary.PrintString` (`self.ZoneWithString` "Player Left " (`self.Zone`))))

(event `PlayerEnteredResponse`
  (bind _gamemode_reference (`self.GameMode Reference`))
  (`KismetSystemLibrary.PrintString` (`self.ZoneWithString` "Player entered" (`self.Zone`)))
  (`self.SimplifiedEZoneSwitch` (`self.Zone`)
    (:`Pathway`
      (`/Game/Character_Folder/Blueprints/BP_FragGameMode.TriggerPathway` _gamemode_reference))
    (:`AltarN`
      (if (not (`self.Latched`))
        (set `self.Latched` true)
        (`self.IncreaseAltarState`)))
    (:`Church`
      (`/Game/Character_Folder/Blueprints/BP_FragGameMode.Trigger_Boss_Sequence` _gamemode_reference))))

(event `FinishZoneResponse`
  (bind (_value _returnvalue) (`BlueprintMapLibrary.Map_Find` (`self.ZoneVolumes`) (`self.Zone`)))
  (if _returnvalue
    (`self.K2_DestroyActor` _value)))

(fn `UserConstructionScript`)

(fn `ZoneWithString`
  (params (Prefix :type String) (Zone :type "/Game/ZoneManager/EZone Enum" :default "NewEnumerator2") (Suffix :type String))
  (returns (ReturnValue :type String))
  (return (`KismetStringLibrary.Concat_StrStr` (`KismetStringLibrary.Concat_StrStr` Prefix (`|GetEnumeratorNameAsString` Zone)) Suffix)))