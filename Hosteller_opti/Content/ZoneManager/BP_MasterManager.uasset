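; BP_MasterManager is an actor that controls which zone is active and signals the zone manager on player transitions.
; ChangeZone lazily finds and caches BP_Zone_Manager, fires its leave call for the old zone, stores the new one, then fires its entered call.
; One enum entry serves as the "no zone" value and skips those calls.
; FinishZone calls the manager's finish, switches to no zone, then calls its unlatched dispatcher.
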(event `self.ReceiveBeginPlay`)

(fn `ChangeZone`
  (params (Zone :type "/Game/ZoneManager/EZone Enum" :default "NewEnumerator2"))
  (bind _zonemanager (`self.ZoneManager` :!label _label)
    (:`then`
      (if (`self.IsValidZone` (`/Game/ZoneManager/BP_Zone_Manager.Zone` _zonemanager))
        (`/Game/ZoneManager/BP_Zone_Manager.PlayerLeave` (`self.ZoneManager`)))
      (bind _output_get (set `/Game/ZoneManager/BP_Zone_Manager.Zone` (`local.Zone`) (`self.ZoneManager`)))
      (if (`self.IsValidZone` _output_get)
        (`/Game/ZoneManager/BP_Zone_Manager.PlayerEntered` (`self.ZoneManager`))))
    (:`else`
      (bind _returnvalue (`GameplayStatics.GetActorOfClass` "/Game/ZoneManager/BP_Zone_Manager.BP_Zone_Manager_C"))
      (set `self.ZoneManager` _returnvalue)
      (goto _label))))

(fn `FinishZone`
  (bind _zonemanager (`self.ZoneManager`))
  (`/Game/ZoneManager/BP_Zone_Manager.FinishZone` _zonemanager)
  (`self.ChangeZone` "NewEnumerator2")
  (`/Game/ZoneManager/BP_Zone_Manager.UnlatchedDispatcher` _zonemanager))

(fn `IsValidZone`
  (params (Zone :type "/Game/ZoneManager/EZone Enum" :default "NewEnumerator2"))
  (returns (ReturnValue :type Boolean))
  (return (`|EnumInequality` Zone "NewEnumerator2")))

(fn `UserConstructionScript`)