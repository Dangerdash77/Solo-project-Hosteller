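; Inventory component for the UI demo that holds the player's items in eight slots and links them to the inventory menu and examination widget.
; It initializes only in Demo_Map, caching player, widget and examination actor references.
; AddItem fills the first empty slot without stacking, and slot edits refresh the matching grid widget.
; DropItem empties a slot and spawns a physics-enabled pickup along a short camera trace, carrying the amount.
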(event `self.ReceiveBeginPlay`
  (bind _returnvalue (`GameplayStatics.GetCurrentLevelName` true))
  (if (`KismetStringLibrary.EqualEqual_StrStr` _returnvalue "Demo_Map")
    (`self.Initialize`)))

(event `Initialize`
  (`KismetArrayLibrary.Array_Resize` (`self.InventorySlots`) 8)
  (bind _asbp_hana (cast `` (`GameplayStatics.GetPlayerCharacter` 0))
    (:`then`
      (set `self.Player Ref` _asbp_hana)
      (set `/Game/UIDemo/Inventory/BPC_Inventory.Inventory Menu Ref` (`/Game/UIDemo/Inventory/BPC_Inventory.Inventory Menu Ref` _asbp_hana) _asbp_hana)
      (bind _returnvalue (`|CreateWidget` "/Game/UIDemo/Inventory/Examination_WB.Examination_WB_C"))
      (set `self.Examination_WBRef` _returnvalue)
      (set `/Game/UIDemo/Inventory/BPC_Inventory.Examination WBRef` (`self.Examination_WBRef`) _asbp_hana)
      ;[1 1 1] Highly Unoptimized
      (bind _returnvalue_2 (`GameplayStatics.GetActorOfClass` "/Game/UIDemo/Inventory/InventoryItems/BP_Examination.BP_Examination_C"))
      (`KismetSystemLibrary.PrintString` (`KismetSystemLibrary.GetObjectName` _returnvalue_2))
      (set `self.BP_ExaminationRef` _returnvalue_2)
      (set `/Game/UIDemo/Inventory/Examination_WB.BPCInventoryRef` self (`self.Examination_WBRef`)))
    (:`CastFailed`
      (`KismetSystemLibrary.PrintString` "Cast Fail"))))

(event `CreateExaminationWidget`
  (params (Index :type Integer))
  (bind _inventory_menu_ref (`/Game/UIDemo/Inventory/BPC_Inventory.Inventory Menu Ref` (`self.Player Ref`)))
  (`/Game/UIDemo/Inventory/Examination_WB.UpdateWidget` (`self.Examination_WBRef`) Index)
  (`Widget.SetVisibility` _inventory_menu_ref "Collapsed")
  (`/Engine/EditorBlueprintResources/StandardMacros.IsValid` (`/Game/UIDemo/Inventory/InventoryMenu_WB.InventoryDropDown_WB` _inventory_menu_ref)
    (:`Is Valid`
      (`/Game/UIDemo/Inventory/InventoryMenu_WB.CloseDropDownMenu` _inventory_menu_ref))
    (:`Is Not Valid`
      _))
  (`UserWidget.AddToViewport` (`self.Examination_WBRef`) 2)
  (set `/Game/UIDemo/Inventory/BPC_Inventory.IsInventoryOpen` false (`self.Player Ref`)))

(fn `AddItem`
  (params (Item :type "/Game/UIDemo/Inventory/InventoryItems/InventoryItem_Master Class Reference") (Amount :type Integer))
  (returns (`Success?` :type Boolean))
  (locals (LocalItem :type "/Game/UIDemo/Inventory/InventoryItems/InventoryItem_Master Class Reference") (LocalAmount :type Integer) (LocalMaxStackAmount :type Integer) (LocalIndex :type Integer :default 0))
  (bind (_success_ _index) (`self.CheckForEmptySlot`))
  (set `local.LocalItem` Item)
  (set `local.LocalAmount` Amount)
  (set `local.LocalMaxStackAmount` (`.MaxStackAmount_8_5464E1FD42189AA1EF667083A9611608` (break `/Game/UIDemo/Inventory/Structs/S_ItemData` (defaults `Object` (`local.LocalItem`)))))
  (if _success_
    (set `local.LocalIndex` _index)
    (`KismetArrayLibrary.Array_Set` (`self.InventorySlots`) (`local.LocalIndex`) (make `/Game/UIDemo/Inventory/Structs/Inventory_Items` (`local.LocalAmount`) (`local.LocalItem`)))
    (`self.UpdateInventorySlot` (`local.LocalIndex`))
    (return true)
    (else
      (`KismetSystemLibrary.PrintString` "No Free Slots!")
      (return false))))

(fn `CheckForEmptySlot`
  (returns (`Success?` :type Boolean) (Index :type Integer))
  (locals (LocalSuccess :type Boolean) (LocalIndex :type Integer))
  (for (_array_element _array_index) (`self.InventorySlots`)
    (if (`KismetSystemLibrary.IsValidClass` (`.Item_7_0C6FDC1340955B1DCB93D5AAFFC040D2` (break `/Game/UIDemo/Inventory/Structs/Inventory_Items` _array_element)))
      (set `local.LocalSuccess` false)
      (else
        (set `local.LocalSuccess` true)
        (set `local.LocalIndex` _array_index)
        (break))))
  (return (`local.LocalSuccess`) (`local.LocalIndex`)))

(fn `Drop Item`
  (params (Index :type Integer))
  (locals (`Local Index` :type Integer) (`Local Amount` :type Integer :default 0) (LocalClass :type "/Game/UIDemo/Inventory/InventoryItems/InventoryItem_Master Class Reference"))
  (bind _camera (`/Game/UIDemo/Inventory/BPC_Inventory.Camera` (`self.Player Ref`)))
  (bind _returnvalue (`SceneComponent.K2_GetComponentLocation` _camera))
  (bind _output_get (set `local.Local Index` Index))
  (bind (_item _amount) (`self.GetItemDataAtIndex` _output_get))
  (set `local.Local Amount` _amount)
  (set `local.LocalClass` _item)
  (if (> (`local.Local Amount`) 0)
    (for _ (range (`local.Local Amount`))
      (`self.RemoveItem` (`local.Local Index`)))
    (`/Game/UIDemo/Inventory/InventoryMenu_WB.CloseDropDownMenu` (`self.Inventory Menu Ref`))
    (bind (_outhit _returnvalue_2) (`KismetSystemLibrary.LineTraceSingle` _returnvalue (+ _returnvalue (* (`SceneComponent.GetForwardVector` _camera) 200.0)) "TraceTypeQuery1"))
    (bind (_bblockinghit _binitialoverlap _time _distance _location _impactpoint _normal _impactnormal _physmat _hitactor _hitcomponent _hitbonename _bonename _hititem _elementindex _faceindex _tracestart _traceend) (`GameplayStatics.BreakHitResult` _outhit))
    (bind _returnvalue_3 (`|SpawnActorFromClass` (`.PickupActor_16_A181F3294F230DFBB0E5AD81C040C366` (break `/Game/UIDemo/Inventory/Structs/S_ItemData` (defaults `Object` (`local.LocalClass`)))) (`KismetMathLibrary.MakeTransform` (select `bool` _returnvalue_2 :`false` _traceend :`true` _location)) "Undefined" "MultiplyWithRoot" null null))
    (set `/Game/UIDemo/Inventory/InventoryItems/PickUpActors/PickUpActor_Master.Amount` (`local.Local Amount`) _returnvalue_3)
    (`PrimitiveComponent.SetSimulatePhysics` (`/Game/UIDemo/Inventory/InventoryItems/PickUpActors/PickUpActor_Master.StaticMesh` _returnvalue_3) true)))

(fn `GetItemDataAtIndex`
  (params (Index :type Integer))
  (returns (Item :type "/Game/UIDemo/Inventory/InventoryItems/InventoryItem_Master Class Reference") (Amount :type Integer))
  (bind (_amount _item) (break `/Game/UIDemo/Inventory/Structs/Inventory_Items` (`|GetArrayItem` (`self.InventorySlots`) Index)))
  (return _item _amount))

(fn `RemoveItem`
  (params (Index :type Integer))
  (bind (_item _amount) (`self.GetItemDataAtIndex` Index))
  (if (> _amount 1)
    (`KismetArrayLibrary.Array_Set` (`self.InventorySlots`) Index (make `/Game/UIDemo/Inventory/Structs/Inventory_Items` (- _amount 1) _item))
    (else
      (`KismetArrayLibrary.Array_Set` (`self.InventorySlots`) Index (make `/Game/UIDemo/Inventory/Structs/Inventory_Items` 0 null))))
  (`self.UpdateInventorySlot` Index))

(fn `UpdateInventorySlot`
  (params (Index :type Integer))
  (`/Game/UIDemo/Inventory/InventorySlot_WB.UpdateSlot` (`|GetArrayItem` (`/Game/UIDemo/Inventory/InventoryGrid_WB.SlotsArray` (`/Game/UIDemo/Inventory/InventoryMenu_WB.InventoryGrid_WB` (`/Game/UIDemo/Inventory/BPC_Inventory.Inventory Menu Ref` (cast `` (`GameplayStatics.GetPlayerCharacter` 0) :!pure true)))) Index)))